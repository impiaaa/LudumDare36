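; EndGame is a trigger actor that ends the game with an explosion when a controlled pawn overlaps it.
; The overlap checks that the other actor's instigator is controlled, then plays a sound and spawns explosion particles both attached to and at the collision component.
; It starts a held camera fade and sets a timer of the same Duration that quits the game when it fires.
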(event `self.ReceiveActorBeginOverlap`
  (params (OtherActor :type "Actor Object Reference"))
  (bind _duration (`self.Duration`))
  (if (`Pawn.IsControlled` (`Actor.Instigator` OtherActor))
    (`GameplayStatics.SpawnSoundAttached` "/Game/StarterContent/Audio/Explosion01.Explosion01" (`self.CollisionComponent`))
    (bind _returnvalue (`GameplayStatics.SpawnEmitterAttached` "/Game/StarterContent/Particles/P_Explosion.P_Explosion" (`self.CollisionComponent`) "None" (0.0 0.0 0.0) (struct) "KeepRelativeOffset" false))
    (`ActorComponent.Activate` _returnvalue true)
    (`PlayerCameraManager.StartCameraFade` :`self` (`GameplayStatics.GetPlayerCameraManager` 0) :`ToAlpha` 1.0 :`Duration` _duration :`bHoldWhenFinished` true)
    (`GameplayStatics.SpawnEmitterAtLocation` "/Game/StarterContent/Particles/P_Explosion.P_Explosion" (`SceneComponent.K2_GetComponentLocation` (`self.CollisionComponent`)))
    (`KismetSystemLibrary.K2_SetTimerDelegate` (delegate `CustomEvent_0`) _duration)))

(event `CustomEvent_0`
  (`KismetSystemLibrary.QuitGame` null "Quit"))

(fn `UserConstructionScript`)