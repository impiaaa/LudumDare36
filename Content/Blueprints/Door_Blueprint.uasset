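; Sliding door that opens when its bound Open event fires, disabling mesh collision and playing an attached sound.
; Opening starts a one-second, non-looping timer with an empty callback, used only as a clock.
; Every Tick offsets the mesh along local X by the timer's elapsed time times a constant, so motion accelerates while the timer runs and depends on frame rate.
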(event `self.ReceiveBeginPlay`
  (add `self.Open` (delegate `Open_Event`)))

(event `Open_Event`
  (bind _staticmeshcomponent (`self.StaticMeshComponent`))
  (`PrimitiveComponent.SetCollisionEnabled` _staticmeshcomponent "NoCollision")
  (`GameplayStatics.SpawnSoundAttached` "/Game/Audio/open.open" _staticmeshcomponent)
  (bind _returnvalue (`KismetSystemLibrary.K2_SetTimerDelegate` (delegate `Timer`) 1.0)))

(event `Timer`)

(event `self.ReceiveTick`
  (params (DeltaSeconds :type "Float (single-precision)"))
  (`SceneComponent.K2_AddLocalOffset` (`self.StaticMeshComponent`) (`KismetMathLibrary.MakeVector` (* (`KismetSystemLibrary.K2_GetTimerElapsedTimeHandle` (stale `Open_Event` _returnvalue)) 10.0)) false false))

(fn `UserConstructionScript`)